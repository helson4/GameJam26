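; BP_Beam is a short-lived beam weapon actor that deals repeated line-trace damage ahead of its owner.
; On BeginPlay it starts firing, sends the owner a lock-movement message, then after two seconds unlocks it and destroys itself.
; FireBeam traces the Visibility channel along the owner's forward vector, damages the hit actor and re-calls itself after a short delay while BeamActive is set.
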(event Custom|FireBeam
  (bind _returnvalue (Components|GetOwner))
  (bind _returnvalue_2 (Transformation|GetActorLocation _returnvalue))
  ;[0.15 0.15 0.15 0.5] Fire Beam
  (bind _outhit (Collision|LineTraceByChannel _returnvalue_2 (+ _returnvalue_2 (* (Variables|Default|GetRange) (Transformation|GetActorForwardVector _returnvalue))) "TraceTypeQuery1" false 0 "None"))
  (Game|Damage|ApplyDamage (.HitActor (Collision|BreakHitResult _outhit)) (Variables|Default|GetDamage) 0 (Variables|Default|GetOwnerCharacter))
  (Utilities|FlowControl|Delay 0.2)
  (if (Variables|Default|GetBeamActive)
    (CallFunction|FireBeam)))

(event EventBeginPlay
  (bind _returnvalue (Components|GetOwner))
  ;[0.15 0.15 0.15 0.5] BeamStart
  (Utilities|Time|SetTimerbyEvent 0 0.1 true)
  (Development|PrintString (Utilities|String|ToString(Vector) (Transformation|GetActorLocation)))
  (Variables|Default|SetBeamActive true)
  (CallFunction|FireBeam)
  (Class|BeamUser|LockMovement(Message) _returnvalue)
  (Utilities|FlowControl|Delay 2.0)
  (Class|BeamUser|UnlockMovement(Message) _returnvalue)
  (Actor|DestroyActor))

(fn ConstructionScript)